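; Invincibility power-up actor that makes the target actor invincible for a set duration.
; ApplyEffect stores the target, sends it an invincibility message, then hides the mesh and disables the collider's physics and collision.
; The hidden actor stays alive until a one-shot timer fires Deactivate, which turns invincibility off and destroys the power-up.
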(event `self.ApplyEffect`
  (params (Actor :type "Actor Object Reference"))
  (bind _collider (`self.Collider`))
  (bind _output_get (set `self.Target` Actor))
  (message `/Game/Exam_UE_2024/Blueprints/Player/I_PlayerFunc.SetInvincible` _output_get true)
  (`PrimitiveComponent.SetSimulatePhysics` _collider false)
  (`PrimitiveComponent.SetCollisionEnabled` _collider "NoCollision")
  (`SceneComponent.SetVisibility` (`self.StaticMesh`) false false)
  (`KismetSystemLibrary.K2_SetTimerDelegate` (delegate `Deactivate`) (`self.Duration`)))

(event `Deactivate`
  (message `/Game/Exam_UE_2024/Blueprints/Player/I_PlayerFunc.SetInvincible` (`self.Target`) false)
  (`self.K2_DestroyActor`))

(fn `UserConstructionScript`
  (`parent.UserConstructionScript`))