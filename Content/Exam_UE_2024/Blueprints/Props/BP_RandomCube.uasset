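; BP_RandomCube is a breakable prop that spawns a drop when the player hits it from below or level.
; On a Collider hit, it checks that the other actor implements I_PlayerFunc and that its location is no higher than the cube's.
; It then passes its drop types, drop rates and location to the game mode's SpawnDropWrapperMessage and destroys itself.
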(event `self.ReceiveBeginPlay`)

(event `self.Collider.OnComponentHit`
  (params (HitComponent :type "PrimitiveComponent Object Reference") (OtherActor :type "Actor Object Reference") (OtherComp :type "PrimitiveComponent Object Reference") (NormalImpulse :type "Vector Structure") (Hit :type "HitResult Structure (by ref)"))
  (bind (_returnvalue_x _returnvalue_y _returnvalue_z) (`KismetMathLibrary.BreakVector` (`KismetMathLibrary.Normal` (- (`self.K2_GetActorLocation` OtherActor) (`self.K2_GetActorLocation`)))))
  (if (`KismetSystemLibrary.DoesImplementInterface` OtherActor "/Game/Exam_UE_2024/Blueprints/Player/I_PlayerFunc.I_PlayerFunc_C")
    (if (<= _returnvalue_z 0.0)
      (message `/Game/Exam_UE_2024/Blueprints/GameMode/GameplayScene/I_GameplayFunc.SpawnDropWrapper` (`GameplayStatics.GetGameMode`) (`self.DropTypes`) (`self.DropRates`) (`self.K2_GetActorLocation`))
      (`self.K2_DestroyActor`))))

(fn `UserConstructionScript`)