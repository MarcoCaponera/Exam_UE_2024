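; Double door prop that swings open once all of its registered conditions are complete.
; AddCondition appends a false flag to the Conditions array, and CompleteCondition sets one true, then ANDs them all.
; If any remain false, successive swaps rotate the array and OpenChecker resets for the next check.
; Open plays a timeline that lerps both door leaves between start and end relative rotations.
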(event `/Game/Exam_UE_2024/Blueprints/Props/Door/I_DoorFunc.AddCondition`
  (`KismetArrayLibrary.Array_Add` (`self.Conditions`)))

(event `Open`
  (bind (_direction _alpha) (`Timeline|TL_Open`)
    (:`Update`
      (`SceneComponent.K2_SetRelativeRotation` (`self.LeftDoor`) (`KismetMathLibrary.RLerp` (`self.LeftStartRot`) (`self.LeftEndRot`) _alpha true) false false)
      (`SceneComponent.K2_SetRelativeRotation` (`self.RightDoor`) (`KismetMathLibrary.RLerp` (`self.RightStartRot`) (`self.RightEndRot`) _alpha true) false false))))

(event `/Game/Exam_UE_2024/Blueprints/Props/Door/I_DoorFunc.CompleteCondition`
  (bind _conditions (`self.Conditions`))
  (`KismetArrayLibrary.Array_Set` _conditions 0 true)
  (for _array_element _conditions
    (set `self.OpenChecker` (and (`self.OpenChecker`) _array_element)))
  (if (`self.OpenChecker`)
    (`self.Open`)
    (else
      (for _index (range (+ (- (`KismetArrayLibrary.Array_Length` (`self.Conditions`)) 2) 1))
        (`KismetArrayLibrary.Array_Swap` (`self.Conditions`) _index (+ _index 1))
        (set `self.OpenChecker` true)))))

(fn `UserConstructionScript`)