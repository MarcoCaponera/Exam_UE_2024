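; BP_EnemyRoom is a room Blueprint whose door condition completes once enough enemies are killed.
; CheckSpecific counts each supplied actor that implements I_EnemyFunc toward Objective.
; KillEnemy increments Progress and sends CompleteConditionMessage to the Door when the count matches Objective.
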(event `self.CheckSpecific`
  (params (Actor :type "Actor Object Reference"))
  (if (`KismetSystemLibrary.DoesImplementInterface` Actor "/Game/Exam_UE_2024/Blueprints/Enemy/I_EnemyFunc.I_EnemyFunc_C")
    (`/Engine/EditorBlueprintResources/StandardMacros.IncrementInt` (`self.Objective`))))

(event `/Game/Exam_UE_2024/Blueprints/Rooms/I_EnemyRoomFunc.KillEnemy`
  (bind _result (`/Engine/EditorBlueprintResources/StandardMacros.IncrementInt` (`self.Progress`))
    (:`  `
      (if (== _result (`self.Objective`))
        (message `/Game/Exam_UE_2024/Blueprints/Props/Door/I_DoorFunc.CompleteCondition` (`self.Door`))))))

(fn `UserConstructionScript`
  (`parent.UserConstructionScript`))