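; BP_RoomBase is a base room actor that links a room's objective to a door and tracks player presence.
; After a short delay at BeginPlay it scans its Area, registers a condition on door-interface actors and passes others to an empty CheckSpecific hook.
; If Objective already equals Progress, it completes the door condition.
; Player overlaps update the GameMode's current room and call empty hooks.
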(event `self.ReceiveBeginPlay`
  (`KismetSystemLibrary.Delay` 0.5)
  (for _array_element (`PrimitiveComponent.GetOverlappingActors` (`self.Area`) null)
    (if (`KismetSystemLibrary.DoesImplementInterface` _array_element "/Game/Exam_UE_2024/Blueprints/Props/Door/I_DoorFunc.I_DoorFunc_C")
      (bind _output_get (set `self.Door` _array_element))
      (message `/Game/Exam_UE_2024/Blueprints/Props/Door/I_DoorFunc.AddCondition` _output_get)
      (else
        (`self.CheckSpecific` _array_element))))
  (`self.AfterBeginPlay`))

(event `OnOverlap`)

(event `OnEndOverlap`)

(event `Setup`)

(event `CheckSpecific`
  (params (Actor :type "Actor Object Reference")))

(event `Restart`)

(event `self.Area.OnComponentBeginOverlap`
  (params (OverlappedComponent :type "PrimitiveComponent Object Reference") (OtherActor :type "Actor Object Reference") (OtherComp :type "PrimitiveComponent Object Reference") (OtherBodyIndex :type Integer) (bFromSweep :type Boolean) (SweepResult :type "HitResult Structure (by ref)"))
  (if (`self.ActorHasTag` OtherActor "Player")
    (message `/Game/Exam_UE_2024/Blueprints/GameMode/GameplayScene/I_GameplayFunc.AddCurrentRoom` (`GameplayStatics.GetGameMode`) self)
    (`self.OnOverlap`)))

(event `self.Area.OnComponentEndOverlap`
  (params (OverlappedComponent :type "PrimitiveComponent Object Reference") (OtherActor :type "Actor Object Reference") (OtherComp :type "PrimitiveComponent Object Reference") (OtherBodyIndex :type Integer))
  (if (`self.ActorHasTag` OtherActor "Player")
    (message `/Game/Exam_UE_2024/Blueprints/GameMode/GameplayScene/I_GameplayFunc.RemoveCurrentRoom` (`GameplayStatics.GetGameMode`) self)
    (`self.OnEndOverlap`)))

(event `Complete`
  (message `/Game/Exam_UE_2024/Blueprints/Props/Door/I_DoorFunc.CompleteCondition` (`self.Door`)))

(event `AfterBeginPlay`
  (if (== (`self.Objective`) (`self.Progress`))
    (`self.Complete`)))

(fn `UserConstructionScript`)