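; BP_EnemyBase is the base enemy character, which hurts the player on contact and dies when stomped from above.
; A HitBox overlap compares the normalized direction to the player: a high Z kills the enemy and knocks the player back, otherwise it deals cooldown-gated damage.
; Death ragdolls the mesh with an impulse, notifies the GameMode, detaches the controller and destroys the actor after a delay.
; It also exposes behavior, movement speed and looping patrol points.
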(event `self.HitBox.OnComponentBeginOverlap`
  (params (OverlappedComponent :type "PrimitiveComponent Object Reference") (OtherActor :type "Actor Object Reference") (OtherComp :type "PrimitiveComponent Object Reference") (OtherBodyIndex :type Integer) (bFromSweep :type Boolean) (SweepResult :type "HitResult Structure (by ref)"))
  (bind (_returnvalue_x _returnvalue_y _returnvalue_z) (`KismetMathLibrary.BreakVector` (`KismetMathLibrary.Normal` (- (`self.K2_GetActorLocation` OtherActor) (`self.K2_GetActorLocation`)))))
  (if (`self.ActorHasTag` OtherActor "Player")
    (if (>= _returnvalue_z 0.7)
      (`self.OnDeath`)
      (message `/Game/Exam_UE_2024/Blueprints/Player/I_PlayerFunc.KnockBack` OtherActor (`self.KnockBackForce`))
      (elif (`self.CanInflictDamage?`)
        (message `/Game/Exam_UE_2024/Blueprints/Player/I_PlayerFunc.TakeDamage` OtherActor)
        (set `self.CanInflictDamage?` false)
        (`KismetSystemLibrary.K2_SetTimerDelegate` (delegate `ResetCanInflictDamage`) (`self.DamageCooldown`))))))

(event `ResetCanInflictDamage`
  (set `self.CanInflictDamage?` true))

(event `OnDeath`
  (`ActorComponent.K2_DestroyComponent` (`self.CapsuleComponent`))
  (`ActorComponent.K2_DestroyComponent` (`self.HitBox`))
  (`PrimitiveComponent.SetSimulatePhysics` (`self.Mesh`) true)
  (`PrimitiveComponent.SetCollisionProfileName` (`self.Mesh`) "Ragdoll" true)
  (`PrimitiveComponent.AddImpulse` (`self.Mesh`) (`self.DeathImpulse`) "None" true)
  (`KismetSystemLibrary.K2_SetTimerDelegate` (delegate `Vanish`) (`self.VanishTime`))
  (message `/Game/Exam_UE_2024/Blueprints/GameMode/GameplayScene/I_GameplayFunc.KillEnemy` (`GameplayStatics.GetGameMode`))
  (`self.DetachFromAI`))

(event `Vanish`
  (`self.K2_DestroyActor`))

(event `/Game/Exam_UE_2024/Blueprints/Enemy/I_EnemyFunc.NotifyPointReached`
  (bind _result (`/Engine/EditorBlueprintResources/StandardMacros.IncrementInt` (`self.CurrentPtr`))
    (:`  `
      (if (== _result (`KismetArrayLibrary.Array_Length` (`self.PointsToReach`)))
        (set `self.CurrentPtr` 0)))))

(event `DetachFromAI`
  (`self.DetachFromControllerPendingDestroy`))

(event `/Game/Exam_UE_2024/Blueprints/Enemy/I_EnemyFunc.SetMovSpeed`
  (params (MovSpeed :type "Float (double-precision)"))
  (set `CharacterMovementComponent.MaxWalkSpeed` MovSpeed (`self.CharacterMovement`)))

(fn `GetBehavior`
  (returns (Behavior :type "BehaviorTree Object Reference"))
  (return (`self.Behavior`)))

(fn `GetPointToReach`
  (returns (Ptr :type "Actor Object Reference"))
  (return (`|GetArrayItem` (`self.PointsToReach`) (`self.CurrentPtr`))))

(fn `UserConstructionScript`)