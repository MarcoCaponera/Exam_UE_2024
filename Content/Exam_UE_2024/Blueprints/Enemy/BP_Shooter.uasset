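; Enemy shooter that attaches its Gun component to the mesh's grip socket on BeginPlay and fires hitscan shots.
; Shoot projects an endpoint at Range toward the target's position, then waits ShootTimeOffset, so the aim is locked before firing.
; It then spawns a muzzle effect and runs a debug-drawn Visibility trace from the muzzle, sending TakeDamageMessage to hit actors implementing I_PlayerFunc.
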(event `self.ReceiveBeginPlay`
  (`parent.ReceiveBeginPlay`)
  (`SceneComponent.K2_AttachToComponent` (`self.Gun`) (`self.Mesh`) "wp_grip" "SnapToTarget" "SnapToTarget" "KeepRelative" true))

(event `/Game/Exam_UE_2024/Blueprints/Enemy/I_ShooterFunc.Shoot`
  (params (ShootAt :type "Actor Object Reference"))
  (bind _returnvalue (`self.K2_GetActorLocation`))
  (bind _returnvalue_2 (`SceneComponent.GetSocketLocation` (`self.Gun`) (`self.MuzzleSocketName`)))
  (set `self.ShootAt` (+ (* (`KismetMathLibrary.Normal` (- (`self.K2_GetActorLocation` ShootAt) _returnvalue)) (`self.Range`)) _returnvalue))
  (`KismetSystemLibrary.Delay` (`self.ShootTimeOffset`))
  (`GameplayStatics.SpawnEmitterAtLocation` "/Game/StarterContent/Particles/P_Explosion.P_Explosion" _returnvalue_2 (struct) (0.3 0.3 0.3))
  (bind _outhit (`KismetSystemLibrary.LineTraceSingle` :`Start` _returnvalue_2 :`End` (`self.ShootAt`) :`TraceChannel` "TraceTypeQuery1" :`DrawDebugType` "ForDuration"))
  (if (`KismetSystemLibrary.DoesImplementInterface` (`.HitActor` (`GameplayStatics.BreakHitResult` _outhit)) "/Game/Exam_UE_2024/Blueprints/Player/I_PlayerFunc.I_PlayerFunc_C")
    (message `/Game/Exam_UE_2024/Blueprints/Player/I_PlayerFunc.TakeDamage` (`.HitActor` (`GameplayStatics.BreakHitResult` _outhit)))))

(fn `UserConstructionScript`
  (`parent.UserConstructionScript`))