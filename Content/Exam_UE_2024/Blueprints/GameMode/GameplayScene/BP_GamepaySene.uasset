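; BP_GamepaySene is a gameplay scene controller that tracks the active room and handles level restart.
; On BeginPlay it sets game-only input for the player.
; SetCurrentRoom stores the given room and runs its Setup, and CollectCoin forwards coin pickups to that room through CollectCoinMessage.
; Restart reopens the current level by name.
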(event `self.ReceiveBeginPlay`
  (`WidgetBlueprintLibrary.SetInputMode_GameOnly` (`GameplayStatics.GetPlayerController` 0)))

(event `/Game/Exam_UE_2024/Blueprints/GameMode/GameplayScene/I_GameplayFunc.CollectCoin`
  (message `/Game/Exam_UE_2024/Blueprints/Rooms/I_CoinRoomFunc.CollectCoin` (`self.CurrentRoom`)))

(event `/Game/Exam_UE_2024/Blueprints/GameMode/GameplayScene/I_GameplayFunc.SetCurrentRoom`
  (params (Room :type "/Game/Exam_UE_2024/Blueprints/Rooms/BP_RoomBase Object Reference"))
  (bind _output_get (set `self.CurrentRoom` Room))
  (`/Game/Exam_UE_2024/Blueprints/Rooms/BP_RoomBase.Setup` _output_get))

(event `/Game/Exam_UE_2024/Blueprints/GameMode/GameplayScene/I_GameplayFunc.Restart`
  (bind _returnvalue (`GameplayStatics.GetCurrentLevelName` true))
  (`GameplayStatics.OpenLevel` (`KismetStringLibrary.Conv_StringToName` _returnvalue)))

(fn `UserConstructionScript`)