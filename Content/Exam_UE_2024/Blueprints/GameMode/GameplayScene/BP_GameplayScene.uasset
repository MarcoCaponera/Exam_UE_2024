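; BP_GameplayScene is a gameplay coordinator that tracks the active rooms and relays game events to them.
; Rooms are set up when added to the CurrentRoom list, and every listed room receives coin-collection, enemy-kill and restart calls.
; On BeginPlay it sets game-only input and caches the level's BP_Spawner, to which it forwards drop spawn requests with types, rates and location.
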(event `self.ReceiveBeginPlay`
  (`WidgetBlueprintLibrary.SetInputMode_GameOnly` (`GameplayStatics.GetPlayerController` 0))
  (bind _returnvalue (`GameplayStatics.GetActorOfClass` "/Game/Exam_UE_2024/Blueprints/Props/Spawner/BP_Spawner.BP_Spawner_C"))
  (set `self.Spawner` _returnvalue))

(event `/Game/Exam_UE_2024/Blueprints/GameMode/GameplayScene/I_GameplayFunc.CollectCoin`
  (for _array_element (`self.CurrentRoom`)
    (message `/Game/Exam_UE_2024/Blueprints/Rooms/I_CoinRoomFunc.CollectCoin` _array_element)))

(event `/Game/Exam_UE_2024/Blueprints/GameMode/GameplayScene/I_GameplayFunc.KillEnemy`
  (for _array_element (`self.CurrentRoom`)
    (message `/Game/Exam_UE_2024/Blueprints/Rooms/I_EnemyRoomFunc.KillEnemy` _array_element)))

(event `/Game/Exam_UE_2024/Blueprints/GameMode/GameplayScene/I_GameplayFunc.AddCurrentRoom`
  (params (Room :type "/Game/Exam_UE_2024/Blueprints/Rooms/BP_RoomBase Object Reference"))
  (`KismetArrayLibrary.Array_Add` (`self.CurrentRoom`) Room)
  (`/Game/Exam_UE_2024/Blueprints/Rooms/BP_RoomBase.Setup` Room))

(event `/Game/Exam_UE_2024/Blueprints/GameMode/GameplayScene/I_GameplayFunc.Restart`
  (for _array_element (`self.CurrentRoom`)
    (`/Game/Exam_UE_2024/Blueprints/Rooms/BP_RoomBase.Restart` _array_element)))

(event `/Game/Exam_UE_2024/Blueprints/GameMode/GameplayScene/I_GameplayFunc.RemoveCurrentRoom`
  (params (Room :type "/Game/Exam_UE_2024/Blueprints/Rooms/BP_RoomBase Object Reference"))
  (`KismetArrayLibrary.Array_RemoveItem` (`self.CurrentRoom`) Room))

(event `/Game/Exam_UE_2024/Blueprints/GameMode/GameplayScene/I_GameplayFunc.SpawnDropWrapper`
  (params (Types :type "Array of /Game/Exam_UE_2024/Blueprints/Props/E_DropTypes Enum (by ref)" :default _) (DropRates :type "Array of Integer (by ref)") (Location :type "Vector Structure"))
  (`/Game/Exam_UE_2024/Blueprints/Props/Spawner/BP_Spawner.SpawnDrop` (`self.Spawner`) Types DropRates Location))

(fn `UserConstructionScript`)