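; BP_Menu is the menu controller Blueprint that manages which widget screen is shown.
; On BeginPlay it adds WB_StartScreen to the viewport, shows the mouse cursor, sets UI-only input focused on that widget, and stores it as CurrentScreen.
; The ChangeWB event swaps screens by removing CurrentScreen, then creating, displaying and storing a widget of the given class, without resetting input focus.
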(event `self.ReceiveBeginPlay`
  (bind _returnvalue (`GameplayStatics.GetPlayerController` 0))
  (bind _returnvalue_2 (`|CreateWidget` "/Game/Exam_UE_2024/UI/StartScreen/Widgets/WB_StartScreen.WB_StartScreen_C"))
  (`UserWidget.AddToViewport` _returnvalue_2 0)
  (set `PlayerController.bShowMouseCursor` true _returnvalue)
  (`WidgetBlueprintLibrary.SetInputMode_UIOnlyEx` _returnvalue _returnvalue_2)
  (set `self.CurrentScreen` _returnvalue_2))

(event `/Game/Exam_UE_2024/Blueprints/GameMode/Menu/I_MenuFunc.ChangeWB`
  (params (WB :type "UserWidget Class Reference"))
  (`Widget.RemoveFromParent` (`self.CurrentScreen`))
  (bind _returnvalue (`|CreateWidget` WB))
  (`UserWidget.AddToViewport` _returnvalue 0)
  (set `self.CurrentScreen` _returnvalue))

(fn `UserConstructionScript`)